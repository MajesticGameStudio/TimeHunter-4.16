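; Car obstacle for a mobile sprite game that stops the Scientist on contact and restarts the level.
; On BeginPlay it picks a random sprite from its Cars array for the car's visual.
; On overlap it hides the Scientist's sprite, zeroes walk speed and jump velocity, then reloads the current level by name after a short delay.
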(event `self.ReceiveActorBeginOverlap`
  (params (OtherActor :type "Actor Object Reference"))
  (bind _asscientist (cast `/Game/Mobile/Blueprints/Scientist` OtherActor))
  (`SceneComponent.SetVisibility` (`PaperCharacter.Sprite` _asscientist) false false)
  (`|ExecutionSequence`
    (:`then_0`
      (bind _charactermovement (`Character.CharacterMovement` _asscientist))
      (set `CharacterMovementComponent.MaxWalkSpeed` 0.0 _charactermovement))
    (:`then_1`
      (set `CharacterMovementComponent.JumpZVelocity` 0.0 _charactermovement)))
  (`KismetSystemLibrary.Delay` 1.0)
  (bind _returnvalue (`GameplayStatics.GetCurrentLevelName` true))
  (`GameplayStatics.OpenLevel` (`KismetStringLibrary.Conv_StringToName` _returnvalue)))

(event `self.ReceiveBeginPlay`
  (bind _cars (`self.Cars`))
  (`PaperSpriteComponent.SetSprite` (`self.Car_Sprite_3`) (`|GetArrayItem` _cars (`KismetMathLibrary.RandomIntegerInRange` 0 (`KismetArrayLibrary.Array_LastIndex` _cars)))))

(fn `UserConstructionScript`)