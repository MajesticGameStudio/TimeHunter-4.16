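; Scientist is the Paper2D player character of a mobile endless runner, auto-running right after a three-second hidden start.
; Tick updates instance-supplied flipbooks, ramps speed and play rate via delayed increments, and calls ZERO.
; Jump input or touch triggers jumps; only touch counts toward MaxJump, reset on landing.
; ZERO treats zero velocity after four seconds as run end: portal flash, best-score save, Lvlend widget; Score-counting logic is disconnected.
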(event `ZERO`
  (bind _charactermovement (`self.CharacterMovement`))
  (bind _score (`self.Score`))
  (if (> (`self.GetGameTimeSinceCreation` (`GameplayStatics.GetGameMode`)) 4.0)
    (if (== (`KismetMathLibrary.VSize` (`self.GetVelocity`)) 0.0)
      (bind _asrun_gm (cast `/Game/Mobile/Blueprints/RunGM` (`GameplayStatics.GetGameMode`)))
      (set `/Game/Mobile/Blueprints/RunGM.ScoreDelay` 5.0 _asrun_gm)
      (bind _asinstance (cast `/Game/Mobile/Blueprints/Instance` (`GameplayStatics.GetGameInstance`)))
      (`|ExecutionSequence`
        (:`then_0`
          (`SceneComponent.SetVisibility` (`self.Sprite`) false false)
          (`|ExecutionSequence`
            (:`then_0`
              (set `CharacterMovementComponent.MaxWalkSpeed` 0.0 _charactermovement))
            (:`then_1`
              (set `CharacterMovementComponent.JumpZVelocity` 0.0 _charactermovement)))
          (`KismetSystemLibrary.Delay` 1.0)
          (bind _returnvalue (`|CreateWidget` "/Game/Mobile/Blueprints/lvlend.lvlend_C"))
          (`UserWidget.AddToViewport` _returnvalue 0))
        (:`then_1`
          (if (>= _score (`/Game/Mobile/Blueprints/Instance.NewScore` _asinstance))
            (set `/Game/Mobile/Blueprints/Instance.NewScore` _score _asinstance)))
        (:`then_2`
          (`SceneComponent.SetVisibility` (`self.Portal_close`) true false)
          (`KismetSystemLibrary.Delay` 0.25)
          (`SceneComponent.SetHiddenInGame` (`self.Portal_close`) true false))))))

(event `self.ReceiveBeginPlay`
  (bind _charactermovement (`self.CharacterMovement`))
  (set `self.Score` 0)
  (`|ExecutionSequence`
    (:`then_0`
      (`ActorComponent.SetIsReplicated` (`self.Sprite`) true))
    (:`then_1`
      (`SceneComponent.SetVisibility` (`self.Portal_close`) false false))
    (:`then_2`
      (set `CharacterMovementComponent.MaxWalkSpeed` 0.0 _charactermovement)
      (`SceneComponent.SetVisibility` (`self.Sprite`) false false)
      (`self.DisableInput` null)
      (`KismetSystemLibrary.Delay` 3.0)
      (`SceneComponent.SetVisibility` (`self.Sprite`) true false)
      (set `CharacterMovementComponent.MaxWalkSpeed` 140.0 _charactermovement)
      (`self.EnableInput` null)
      (set `self.is moves?` true))))

(event `UpdateAnimation`
  ;[1 1 1] Handle Animation
  (bind _asinstance (cast `/Game/Mobile/Blueprints/Instance` (`GameplayStatics.GetGameInstance`)))
  (if (`|EnumEquality` (`self.State`) "NewEnumerator2")
    (`PaperFlipbookComponent.SetFlipbook` (`self.Sprite`) (`/Game/Mobile/Blueprints/Instance.JumpRef` _asinstance))
    (else
      (bind _flipref (`/Game/Mobile/Blueprints/Instance.FlipRef` _asinstance))
      (`PaperFlipbookComponent.SetFlipbook` (`self.Sprite`) (select `bool` (> (`KismetMathLibrary.VSize` (`self.GetVelocity`)) 0.0) :`false` _flipref :`true` _flipref)))))

(event `self.ReceiveTick`
  (params (DeltaSeconds :type "Float (single-precision)"))
  (bind _charactermovement (`self.CharacterMovement`))
  (bind _sprite (`self.Sprite`))
  (`|ExecutionSequence`
    (:`then_0`
      ;[1 1 1] Tick - Updates animation & SpeedProgress
      (`self.UpdateAnimation`))
    (:`then_1`
      (`self.AddMovementInput` (1.0 0.0 0.0)))
    (:`then_2`
      (`KismetSystemLibrary.Delay` 5.0)
      (set `CharacterMovementComponent.MaxWalkSpeed` (+ (`CharacterMovementComponent.MaxWalkSpeed` _charactermovement) (`self.SpeedProgress`)) _charactermovement)
      (`PaperFlipbookComponent.SetPlayRate` _sprite (+ (`PaperFlipbookComponent.GetPlayRate` _sprite) (`self.RateProg`))))
    (:`then_3`
      (if (== (`CharacterMovementComponent.MaxWalkSpeed` _charactermovement) 200.0)
        (set `self.SpeedProgress` 0.0)))
    (:`then_4`
      (if (== (`PaperFlipbookComponent.GetPlayRate` (`self.Sprite`)) 1.5)
        (set `self.RateProg` 0.0)))
    (:`then_7`
      (`self.ZERO`))))

(event `InputAction|Jump`
  (params (Key :type "Key Structure" :default "AnyKey"))
  ;[1 1 1] Handle Jump
  (:`Pressed`
    (`self.Jump` :!label _label)
    (set `self.State` "NewEnumerator2")
    (`PaperFlipbookComponent.SetFlipbook` (`self.Sprite`) (`self.JumpRef`)))
  (:`Released`
    (`self.StopJumping` :!label _label_2)))

(event `InputTouch`
  (params (Location :type "Vector Structure") (FingerIndex :type "ETouchIndex Enum"))
  (bind _jump_counter (`self.Jump counter`))
  ;[1 1 1] Handle Jump
  (:`Pressed`
    (if (< _jump_counter (`self.Max jump`))
      (set `self.Jump counter` (+ _jump_counter 1))
      (goto _label)))
  (:`Released`
    (goto _label_2)))

(event `self.OnLanded`
  (params (Hit :type "HitResult Structure (by ref)"))
  ;[1 1 1] Handle Jump
  (set `self.Jump counter` 0)
  (set `self.State` "NewEnumerator0"))

(fn `UserConstructionScript`)