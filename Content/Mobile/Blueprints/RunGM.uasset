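; Game mode for a mobile endless runner that builds the track and scenery and counts the Scientist's score.
; On BeginPlay it spawns floor tiles, backdrops and City-only houses by level name (Forest, City, Desert), chaining each piece from the previous one's returned transform.
; Tick raises score through a repeating Delay; speed-based pacing and high-score saving are disconnected.
; A separate helper opens a random level, Forest or Space among them.
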(event `self.ReceiveBeginPlay`
  (`|ExecutionSequence`
    (:`then_0`
      (for _ (range 10)
        (`self.AddFloor`)))
    (:`then_1`
      (for _ (range 4)
        (`self.addBack`)))
    (:`then_2`
      (for _ (range 7)
        (`self.AddEnvir`)))))

(event `self.ReceiveTick`
  (params (DeltaSeconds :type "Float (single-precision)"))
  (`|ExecutionSequence`
    (:`then_1`
      (`KismetSystemLibrary.Delay` (`self.ScoreDelay`))
      (bind _asscientist (cast `/Game/Mobile/Blueprints/Scientist` (`GameplayStatics.GetPlayerCharacter` 0)))
      (set `/Game/Mobile/Blueprints/Scientist.Score` (+ (`/Game/Mobile/Blueprints/Scientist.Score` _asscientist) 1) _asscientist)
      (`/Engine/EditorBlueprintResources/StandardMacros.DoOnce` false
        (:`Completed`
          (set `self.ScoreDelay` 0.15))))
    (:`then_2`
      (bind _asinstance (cast `/Game/Mobile/Blueprints/Instance` (`GameplayStatics.GetGameInstance`))))))

(fn `addBack`
  (bind _returnvalue (`GameplayStatics.GetCurrentLevelName` true))
  (`|ExecutionSequence`
    (:`then_0`
      (if (== (`KismetStringLibrary.Conv_StringToName` _returnvalue) "Forest")
        ;[1 1 1] Mountains Back
        (bind _returnvalue_2 (`|SpawnActorFromClass` "/Game/Mobile/Sprites/BackGrounds/Background_mountain_BP.Background_mountain_BP_C" (`self.Nextpoint`) "Undefined" "OverrideRootScale" :!label _label))
        (bind _asbackground_mountain_bp (cast `/Game/Mobile/Sprites/BackGrounds/Background_mountain_BP` _returnvalue_2))
        (bind _newparam (`/Game/Mobile/Sprites/BackGrounds/Background_mountain_BP.GetTrans` _asbackground_mountain_bp))
        (set `self.Nextpoint` _newparam)))
    (:`then_1`
      (if (== (`KismetStringLibrary.Conv_StringToName` _returnvalue) "City")
        (goto _label)))
    (:`then_2`
      (if (`KismetStringLibrary.EqualEqual_StrStr` _returnvalue "Desert")
        (bind _returnvalue_3 (`|SpawnActorFromClass` "/Game/Mobile/Sprites/BackGrounds/Background_desert_bp.Background_desert_BP_C" (`self.Nextpoint`) "Undefined" "OverrideRootScale"))
        (bind _asbackground_desert_bp (cast `/Game/Mobile/Sprites/BackGrounds/Background_desert_bp` _returnvalue_3))
        (bind _newparam_2 (`/Game/Mobile/Sprites/BackGrounds/Background_desert_bp.GetTrans` _asbackground_desert_bp))
        (set `self.Nextpoint` _newparam_2)))))

(fn `AddEnvir`
  (bind _houses (`self.Houses`))
  (bind _returnvalue (`GameplayStatics.GetCurrentLevelName` true))
  (`|ExecutionSequence`
    (:`then_0`
      (if (== (`KismetStringLibrary.Conv_StringToName` _returnvalue) "Forest")
        _))
    (:`then_1`
      (if (== (`KismetStringLibrary.Conv_StringToName` _returnvalue) "City")
        ;[1 1 1] Mountains Back
        (bind _returnvalue_2 (`|SpawnActorFromClass` (`|GetArrayItem` _houses (`KismetMathLibrary.RandomIntegerInRange` 0 (`KismetArrayLibrary.Array_LastIndex` _houses))) (`self.NewVar_0`) "Undefined" "OverrideRootScale"))
        (bind _ashouse_bp_1 (cast `/Game/Mobile/Sprites/Buildings/House_BP_1` _returnvalue_2))
        (bind _newparam (`/Game/Mobile/Sprites/Buildings/House_BP_1.GetTrans` _ashouse_bp_1))
        (set `self.NewVar_0` _newparam)))))

(fn `AddFloor`
  (bind _forest_tiles (`self.Forest Tiles`))
  (bind _deserttiles (`self.DesertTiles`))
  (bind _city_tiles (`self.City Tiles`))
  (bind _returnvalue (`GameplayStatics.GetCurrentLevelName` true))
  (`|ExecutionSequence`
    (:`then_0`
      (if (== (`KismetStringLibrary.Conv_StringToName` _returnvalue) "Forest")
        ;[1 1 1] Forest
        (bind _returnvalue_2 (`|SpawnActorFromClass` (`|GetArrayItem` _forest_tiles (`KismetMathLibrary.RandomIntegerInRange` 0 (`KismetArrayLibrary.Array_LastIndex` _forest_tiles))) (`self.NEXTSPAWNPOINT`) "Undefined" "OverrideRootScale"))
        (bind _astile_1 (cast `/Game/Mobile/Sprites/Tiles/TILES_Forest/BPs/TILE_1` _returnvalue_2))
        (bind _attachtransform (`/Game/Mobile/Sprites/Tiles/TILES_Forest/BPs/TILE_1.GetAttachTransform` _astile_1))
        (set `self.NEXTSPAWNPOINT` _attachtransform)))
    (:`then_1`
      (if (== (`KismetStringLibrary.Conv_StringToName` _returnvalue) "City")
        ;[1 1 1] City
        (bind _returnvalue_3 (`|SpawnActorFromClass` (`|GetArrayItem` _city_tiles (`KismetMathLibrary.RandomIntegerInRange` 0 (`KismetArrayLibrary.Array_LastIndex` _city_tiles))) (`self.NEXTSPAWNPOINT`) "Undefined" "OverrideRootScale"))
        (bind _astile_bp_city_1 (cast `/Game/Mobile/Sprites/Tiles/TILES_City/TILE_BP_city1` _returnvalue_3))
        (bind _attachtransform_2 (`/Game/Mobile/Sprites/Tiles/TILES_City/TILE_BP_city1.GetAttachTransform` _astile_bp_city_1))
        (set `self.NEXTSPAWNPOINT` _attachtransform_2)))
    (:`then_2`
      (if (`KismetStringLibrary.EqualEqual_StrStr` _returnvalue "Desert")
        ;[1 1 1] City
        (bind _returnvalue_4 (`|SpawnActorFromClass` (`|GetArrayItem` _deserttiles (`KismetMathLibrary.RandomIntegerInRange` 0 (`KismetArrayLibrary.Array_LastIndex` _deserttiles))) (`self.NEXTSPAWNPOINT`) "Undefined" "OverrideRootScale"))
        (bind _astile_des_bp_1 (cast `/Game/Mobile/Sprites/Tiles/TILES_Desert/Tile_des_BP_1` _returnvalue_4))
        (bind _attachtransform_3 (`/Game/Mobile/Sprites/Tiles/TILES_Desert/Tile_des_BP_1.GetAttachTransform` _astile_des_bp_1))
        (set `self.NEXTSPAWNPOINT` _attachtransform_3)))))

(fn `OpenRANDOMLEVEL`
  (switch `int` (`KismetMathLibrary.RandomIntegerInRange` 0 2)
    (:`0`
      (`GameplayStatics.OpenLevel` "Forest"))
    (:`1`
      (`GameplayStatics.OpenLevel` "Space"))))

(fn `UserConstructionScript`)